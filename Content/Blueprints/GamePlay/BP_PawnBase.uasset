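; Base VR pawn that feeds headset movement into motion-platform control through PlatformControlSubsystem, starting its send thread on BeginPlay.
; While the subsystem runs, Tick picks scaled camera rotation or tilt derived via atan2 from camera offset over ZHeight.
; RotationFunction passes absolute roll and pitch differences from PlatformRotation to RotateLogic, defined outside this graph.
; Enhanced Input toggles sending and rotation/location mode, nudges RotateThreshold (seeded from WECGameInstance) and resets HMD origin.
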(event `self.ReceiveBeginPlay`
  (`PlatformControlSubsystem.RunSendThread` (subsystem `PlatformControlSubsystem`))
  (`EnhancedInputSubsystemInterface.AddMappingContext` (pcsubsystem `EnhancedInputLocalPlayerSubsystem` (`GameplayStatics.GetPlayerController` 0)) "/Game/Blueprints/Input/IMC_VRInput.IMC_VRInput" 0 (struct))
  (bind _aswecgame_instance (cast `WECGameInstance` (`GameplayStatics.GetGameInstance`)))
  (set `self.RotateThreshold` (`WECGameInstance.RotateThreshold` _aswecgame_instance))
  (if (`HeadMountedDisplayFunctionLibrary.IsHeadMountedDisplayEnabled`)
    (`HeadMountedDisplayFunctionLibrary.SetTrackingOrigin` "Stage")
    (`KismetSystemLibrary.ExecuteConsoleCommand` "vr.PixelDensity 1.0" null)))

(event `self.ReceiveTick`
  (params (DeltaSeconds :type "Float (single-precision)"))
  (if (`PlatformControlSubsystem.bRunning` (subsystem `PlatformControlSubsystem`))
    (`self.RotationFunction` (`self.SwitchRotateFunction`))))

(event `EnhancedInput|/Game/Blueprints/Input/IA_ControlAngle`
  (params (ActionValue :type "Float (double-precision)") (ElapsedSeconds :type "Float (double-precision)") (TriggeredSeconds :type "Float (double-precision)") (InputAction :type "InputAction Object Reference" :default "/Game/Blueprints/Input/IA_ControlAngle.IA_ControlAngle"))
  (bind _rotatethreshold (`self.RotateThreshold`))
  (:`Started`
    (if (> ActionValue 0.0)
      (`/Engine/EditorBlueprintResources/StandardMacros.IncrementFloat` _rotatethreshold)
      (else
        (`/Engine/EditorBlueprintResources/StandardMacros.DecrementFloat` _rotatethreshold)))))

(event `Key|One`
  (params (Key :type "Key Structure")))

(event `EnhancedInput|/Game/Blueprints/Input/IA_ChangeSendDataToPlatform`
  (params (ActionValue :type Boolean) (ElapsedSeconds :type "Float (double-precision)") (TriggeredSeconds :type "Float (double-precision)") (InputAction :type "InputAction Object Reference" :default "/Game/Blueprints/Input/IA_ChangeSendDataToPlatform.IA_ChangeSendDataToPlatform"))
  (bind _returnvalue (subsystem `PlatformControlSubsystem`))
  (:`Started`
    (`/Engine/EditorBlueprintResources/StandardMacros.FlipFlop`
      (:`A`
        (`PlatformControlSubsystem.RunSendThread` _returnvalue))
      (:`B`
        (`PlatformControlSubsystem.StopSendThread` _returnvalue)))))

(event `EnhancedInput|/Game/Blueprints/Input/IA_ChangeRotOrLoc`
  (params (ActionValue :type Boolean) (ElapsedSeconds :type "Float (double-precision)") (TriggeredSeconds :type "Float (double-precision)") (InputAction :type "InputAction Object Reference" :default "/Game/Blueprints/Input/IA_ChangeRotOrLoc.IA_ChangeRotOrLoc"))
  (:`Started`
    (bind _isa (`/Engine/EditorBlueprintResources/StandardMacros.FlipFlop`)
      (:`A`
        _)
      (:`B`
        _))
    (set `self.bUseRotation` _isa)))

(event `EnhancedInput|/Game/Blueprints/Input/IA_ResetOri`
  (params (ActionValue :type Boolean) (ElapsedSeconds :type "Float (double-precision)") (TriggeredSeconds :type "Float (double-precision)") (InputAction :type "InputAction Object Reference" :default "/Game/Blueprints/Input/IA_ResetOri.IA_ResetOri"))
  (:`Started`
    (`HeadMountedDisplayFunctionLibrary.ResetOrientationAndPosition` 0.0)))

(fn `LocationToRotation`
  (returns (Rotation :type "Rotator Structure"))
  (bind _zheight (`self.ZHeight`))
  (bind (_relativelocation_x _relativelocation_y) (`KismetMathLibrary.BreakVector` (`SceneComponent.RelativeLocation` (`self.VRCamera`))))
  (return (`KismetMathLibrary.MakeRotator` (`KismetStringLibrary.Conv_StringToDouble` (`KismetStringLibrary.Conv_DoubleToString` (`KismetMathLibrary.DegAtan2` _relativelocation_y _zheight))) (`KismetStringLibrary.Conv_StringToDouble` (`KismetStringLibrary.Conv_DoubleToString` (`KismetMathLibrary.DegAtan2` _relativelocation_x _zheight))))))

(fn `RotationFunction`
  (params (CurrentRot :type "Rotator Structure"))
  (bind (_platformrotation_roll _platformrotation_pitch) (`KismetMathLibrary.BreakRotator` (`self.PlatformRotation`)))
  (bind _output_get (set `self.VRCameraRotation` CurrentRot))
  (`|ExecutionSequence`
    (:`then_0`
      (bind _output_get_2 (set `self.PlatformXAngleDifference` (`KismetMathLibrary.Abs` (- (.roll _output_get) _platformrotation_roll))))
      (`self.RotateLogic` _output_get_2 true))
    (:`then_1`
      (bind _output_get_3 (set `self.PlatformYAngleDifference` (`KismetMathLibrary.Abs` (- (.pitch _output_get) _platformrotation_pitch))))
      (`self.RotateLogic` _output_get_3))))

(fn `SwitchRotateFunction`
  (returns (ReturnValue :type "Rotator Structure"))
  (bind (_relativerotation_roll _relativerotation_pitch _relativerotation_yaw) (`KismetMathLibrary.BreakRotator` (`SceneComponent.RelativeRotation` (`self.VRCamera`))))
  (return (`KismetMathLibrary.SelectRotator` (* (`KismetMathLibrary.MakeRotator` _relativerotation_roll (- _relativerotation_pitch 7.0) _relativerotation_yaw) (`self.RotateMult`)) (`self.LocationToRotation`) (`self.bUseRotation`))))

(fn `UserConstructionScript`)